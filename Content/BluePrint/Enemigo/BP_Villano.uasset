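; BP_Villano is an enemy that moves by a constant local offset every Tick, not scaled by delta time, and fires bullets.
; A looping timer calls Disparar, which spawns BP_Bala at the villain's location and rotation while Atacar is true.
; Each shot first multiplies the stored bullet speed by MultVelocidadBala, so speed compounds.
; Setters expose movement, attack state and a hero target, which is stored but unused here.
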(event Custom|Disparar
  (if (Variables|Default|GetAtacar)
    (CallFunction|SetVelocidadBala (Variables|Default|GetVelocidad%20de%20Bala))
    (CallFunction|SpawnBala)))

(event EventBeginPlay
  (Utilities|Time|SetTimerbyEvent (delegate Custom|Disparar) (Variables|Default|GetTiempo%20de%20Disparo) true))

(event EventTick
  (params (DeltaSeconds :type Float%20%28single-precision%29))
  (Transformation|AddActorLocalOffset (Variables|Default|GetVelocidadVillano) false false))

(fn ConstructionScript)

(fn SetVelocidadBala
  (params (NewParam :type Vector))
  (Variables|Default|SetVelocidad%20de%20Bala (* NewParam (Variables|Default|GetMult%20Velocidad%20Bala))))

(fn SpawnBala
  (bind _returnvalue (Transformation|GetActorRotation))
  (Game|SpawnActorfromClass "/Game/BluePrint/BP_Bala.BP_Bala_C" (Math|Transform|MakeTransform (Transformation|GetActorLocation) _returnvalue "1.000000,1.000000,1.000000") "Undefined" "MultiplyWithRoot" 0 (Variables|Default|GetVelocidad%20de%20Bala) _returnvalue 0))

(fn VelocidadVillano
  (params (Velocidad%20Inici :type Vector))
  (Variables|Default|SetVelocidadVillano Velocidad%20Inici))

(fn SetTargetHeroe
  (params (Posición :type Vector))
  (Variables|Default|SetTarget%20Heroe Posición))

(fn SetAtacar
  (params (Atacar :type Boolean))
  (Variables|Default|SetAtacar Atacar))